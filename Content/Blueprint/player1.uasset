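; Player1 Blueprint that moves itself along a spline owned by the level1 object.
; On BeginPlay it casts Level to level1 and caches it as CurLevel, printing a cast-failure message in Chinese otherwise.
; Each Tick it snaps its location and rotation to the spline transform at an accumulated distance, which grows at a fixed, frame-rate-independent speed.
; The distance has no wrap or clamp, and Tick does not check that CurLevel is valid.
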(event `self.ReceiveBeginPlay`
  (bind _aslevel_1 (cast `/Game/Blueprint/level1` (`self.level`))
    (:`then`
      (set `self.CurLevel` _aslevel_1))
    (:`CastFailed`
      (`KismetSystemLibrary.PrintText` "转换失败"))))

(event `self.ReceiveTick`
  (params (DeltaSeconds :type "Float (single-precision)"))
  (bind _length (`self.length`))
  (`self.K2_SetActorLocationAndRotation` (.location (`SplineComponent.GetTransformAtDistanceAlongSpline` (`/Game/Blueprint/level1.Spline` (`self.CurLevel`)) _length "World" false)) (.rotation (`SplineComponent.GetTransformAtDistanceAlongSpline` (`/Game/Blueprint/level1.Spline` (`self.CurLevel`)) _length "World" false)))
  (set `self.length` (+ _length (* DeltaSeconds 100.0))))

(fn `UserConstructionScript`)