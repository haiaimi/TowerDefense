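; Map blueprint that applies bombs across four box components in a timed sequence.
; Its ApplyBomb event passes Box, Box1, Box2 and Box3 in turn to ParentApplyBomb, with a short delay before each call.
; The BeginPlay, overlap and Tick events and the construction script are empty, so ApplyBomb is the only active logic.
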(event `self.ApplyBomb`
  (params (Box :type "BoxComponent Object Reference"))
  (`KismetSystemLibrary.Delay` 1.0)
  (`parent.ApplyBomb` (`self.Box`))
  (`KismetSystemLibrary.Delay` 1.0)
  (`parent.ApplyBomb` (`self.Box1`))
  (`KismetSystemLibrary.Delay` 1.0)
  (`parent.ApplyBomb` (`self.Box2`))
  (`KismetSystemLibrary.Delay` 1.0)
  (`parent.ApplyBomb` (`self.Box3`)))

(fn `UserConstructionScript`)